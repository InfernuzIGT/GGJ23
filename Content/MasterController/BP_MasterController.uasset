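; BP_MasterController runs the game's looping enemy waves and holds a game tick for player income.
; Each round picks a random point inside a random BP_SpawnerCollision and spawns that round's enemy group from DAEnemyGroup.
; Successive spawns step by random offsets alternating between X and Y, and each enemy receives a reference to the controller.
; AddPlayerincome adds to Income, but the tick's GivePlayerIncome and EnemyDeath are empty stubs.
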(event `self.ReceiveBeginPlay`
  (`self.BeginEnemiesGraph`)
  (`self.BeginGameTickGraph`)
  (bind _returnvalue (`GameplayStatics.GetActorOfClass` "/Game/Core/BP_Player.BP_Player_C"))
  (set `self.player` _returnvalue))

(event `EnemyDeath`)

(event `BeginEnemiesGraph`
  (`self.GetSpawnerCollisions`)
  (`self.BeginTimerToEnemyRound`))

(event `GetSpawnerCollisions`
  (bind _outactors (`GameplayStatics.GetAllActorsOfClass` "/Game/Enemies/BP_SpawnerCollision.BP_SpawnerCollision_C"))
  (set `self.SpawnerCollisions` _outactors))

(event `BeginTimerToEnemyRound`
  (`KismetSystemLibrary.K2_SetTimerDelegate` (delegate `EnemyRoundExecute`) (`self.TimeToEnemyRound`) true))

(event `EnemyRoundExecute`
  (`/Engine/EditorBlueprintResources/StandardMacros.IncrementInt` (`self.EnemyRoundCount`)
    (:`  `
      (set `self.tempEnemySpawningPoint` (`/Game/Enemies/BP_SpawnerCollision.GetRandomPointInBoundingBox` (`KismetArrayLibrary.Array_Random` (`self.SpawnerCollisions`))))
      (`self.SpawnEnemyGroup`))))

(event `SpawnEnemyGroup`
  (bind _tempenemyspawningpoint (`self.tempEnemySpawningPoint`))
  (bind _enemygroup (`/Game/Enemies/EnemyGroup/PDA_EnemyGroup.GetEnemyGroup` (`self.DAEnemyGroup`) (`self.EnemyRoundCount`)))
  (for _array_element (`.EnemyList_4_494F16C947A0866B166B5C84991E9F53` (break `/Game/Enemies/EnemyGroup/ST_EnemyGroup` _enemygroup))
    (`|SpawnActorFromClass` _array_element (`KismetMathLibrary.MakeTransform` _tempenemyspawningpoint) "AdjustIfPossibleButAlwaysSpawn" "OverrideRootScale" null self null)
    (bind _isa (`/Engine/EditorBlueprintResources/StandardMacros.FlipFlop`)
      (:`A`
        _)
      (:`B`
        _))
    (set `self.tempEnemySpawningPoint` (+ _tempenemyspawningpoint (select `bool` _isa :`false` (`KismetMathLibrary.MakeVector` (`KismetMathLibrary.RandomFloatInRange` -600.0 600.0)) :`true` (`KismetMathLibrary.MakeVector` 0.0 (`KismetMathLibrary.RandomFloatInRange` -600.0 600.0)))))))

(event `BeginGameTickGraph`
  (`KismetSystemLibrary.K2_SetTimerDelegate` (delegate `GameTickExecute`) (`self.GameTick`) true))

(event `GameTickExecute`
  (`self.GivePlayerIncome`))

(event `GivePlayerIncome`)

(event `AddPlayerincome`
  (params (AddedAmount :type Integer))
  (set `self.income` (+ AddedAmount (`self.income`))))

(fn `UserConstructionScript`)