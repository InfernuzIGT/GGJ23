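; BP_Projectile is a tower projectile that flies toward a target location and damages what it hits.
; On BeginPlay, ProjectileMovement drives the Sphere at high fixed speed in a straight direction toward EndLoc.
; On sphere overlap with any actor not tagged Tower, it applies fixed point damage with an empty hit result and zero direction, then destroys itself.
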(event `self.ReceiveBeginPlay`
  (bind _projectilemovement (`self.ProjectileMovement`))
  (`MovementComponent.SetUpdatedComponent` _projectilemovement (`self.Sphere`))
  (set `MovementComponent.Velocity` (* (`KismetMathLibrary.GetDirectionUnitVector` (`self.K2_GetActorLocation`) (`self.EndLoc`)) 12000.0) _projectilemovement))

(event `self.Sphere.OnComponentBeginOverlap`
  (params (OverlappedComponent :type "PrimitiveComponent Object Reference") (OtherActor :type "Actor Object Reference") (OtherComp :type "PrimitiveComponent Object Reference") (OtherBodyIndex :type Integer) (bFromSweep :type Boolean) (SweepResult :type "HitResult Structure (by ref)"))
  (if (not (`self.ActorHasTag` OtherActor "Tower"))
    (`GameplayStatics.ApplyPointDamage` OtherActor 50.0 (`KismetMathLibrary.MakeVector` 0.0) (`GameplayStatics.MakeHitResult` false) null self)
    (`self.K2_DestroyActor`)))

(fn `UserConstructionScript`)