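; BP_Tower_excavator is an economy tower that raises the player's income for as long as it stands.
; On BeginPlay it fills its health, adds its Income to BP_MasterController and starts a looping timer that spawns a currency-gain Niagara effect above it.
; Point damage reduces health, and at zero the tower subtracts that income again and destroys itself.
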(event `IncreaseAmount`
  (params (Amount :type Integer))
  ;[1 1 1] Increase
  (bind _returnvalue (`GameplayStatics.GetActorOfClass` "/Game/MasterController/BP_MasterController.BP_MasterController_C"))
  (`/Game/MasterController/BP_MasterController.AddPlayerincome` _returnvalue Amount))

(event `self.ReceiveBeginPlay`
  ;[1 1 1] Increase
  (set `self.CurrentHealth` (`self.MaxHealth`))
  (`self.IncreaseAmount` (`self.income`))
  (`KismetSystemLibrary.K2_SetTimerDelegate` (delegate `VFX`) 5.0 true))

(event `VFX`
  (`NiagaraFunctionLibrary.SpawnSystemAtLocation` "/Game/Towers/NS_CurrencyGain.NS_CurrencyGain" (+ (`self.K2_GetActorLocation`) (0.0 0.0 100.0))))

(event `self.ReceivePointDamage`
  (params (Damage :type "Float (single-precision)") (DamageType :type "DamageType Object Reference") (HitLocation :type "Vector Structure") (HitNormal :type "Vector Structure") (HitComponent :type "PrimitiveComponent Object Reference") (BoneName :type Name) (ShotFromDirection :type "Vector Structure") (InstigatedBy :type "Controller Object Reference") (DamageCauser :type "Actor Object Reference") (HitInfo :type "HitResult Structure (by ref)"))
  ;[1 1 1] destroy
  (bind _output_get (set `self.CurrentHealth` (- (`self.CurrentHealth`) Damage)))
  (if (<= _output_get 0.0)
    (`self.IncreaseAmount` (* (`self.income`) -1))
    (`self.K2_DestroyActor`)))

(fn `UserConstructionScript`
  (`parent.UserConstructionScript`))