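; BP_ChildTree is a child Blueprint for a tree that lights up when an actor tagged Tower enters its sphere.
; TurnOn swaps a mesh material to yellow leaves, activates a mystic wisp Niagara effect and reports a found sapling to BP_Player.
; The overlap handler has no once-only guard, so each qualifying overlap reports again.
; Tick prints the names of all overlapping actors as debug output.
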(event `self.ReceiveBeginPlay`
  (`parent.ReceiveBeginPlay`))

(event `TurnOn`
  (`PrimitiveComponent.SetMaterial` (`self.Mesh`) 1 "/Game/Geometry/Materials/OrikamiTree/TreeMat_YellowLeaves_Inst.TreeMat_YellowLeaves_Inst")
  (`ActorComponent.Activate` (`self.NS_MysticWispV2`) true)
  (bind _returnvalue (`GameplayStatics.GetActorOfClass` "/Game/Core/BP_Player.BP_Player_C"))
  (`/Game/Core/BP_Player.AddSaplingFound` _returnvalue))

(event `self.Sphere.OnComponentBeginOverlap`
  (params (OverlappedComponent :type "PrimitiveComponent Object Reference") (OtherActor :type "Actor Object Reference") (OtherComp :type "PrimitiveComponent Object Reference") (OtherBodyIndex :type Integer) (bFromSweep :type Boolean) (SweepResult :type "HitResult Structure (by ref)"))
  (if (`self.ActorHasTag` OtherActor "Tower")
    (`self.TurnOn`)))

(event `self.ReceiveTick`
  (params (DeltaSeconds :type "Float (single-precision)"))
  (for _array_element (`PrimitiveComponent.GetOverlappingActors` (`self.Sphere`) null)
    (`KismetSystemLibrary.PrintString` (`KismetSystemLibrary.GetDisplayName` _array_element))))

(fn `UserConstructionScript`
  (`parent.UserConstructionScript`))