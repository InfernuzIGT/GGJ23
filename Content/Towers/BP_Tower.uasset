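; BP_Tower is a damageable, selectable turret actor that plays a Niagara effect and destroys itself when health runs out.
; UpdateData loads a turret data asset by index to set the mesh, area decal scale and shader line size.
; Selection toggles the decal, while a retriggerable delay briefly pulses a highlight parameter on dynamic mesh materials.
; It also holds a weight, reveals itself after a delayed activation, and can widen a linked branch's root.
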(event `self.ReceiveBeginPlay`
  (bind _mesh (`self.Mesh`))
  (set `self.CurrentHealth` (`self.MaxHealth`))
  (`|ExecutionSequence`
    (:`then_0`
      (for (_array_element _array_index) (`MeshComponent.GetMaterials` _mesh)
        (bind _returnvalue (`PrimitiveComponent.CreateDynamicMaterialInstance` _mesh _array_index _array_element "None"))
        (`KismetArrayLibrary.Array_Add` (`self.Material Mesh`) _returnvalue)))
    (:`then_2`
      (`self.Change Selection State` false)
      (`/Game/Core/BPI_Selection.Update Data` 0))))

(event `Change Selection State`
  (params (bIsSelected :type Boolean))
  (`SceneComponent.SetVisibility` (`self.Decal Area`) bIsSelected false))

(event `Init`
  (bind _returnvalue (`DecalComponent.CreateDynamicMaterialInstance` (`self.Decal Area`)))
  (set `self.Material Area` _returnvalue))

(event `/Game/Core/BPI_Selection.Remove Selection`
  (`self.Change Selection State` false))

(event `/Game/Core/BPI_Selection.Update Data`
  (params (Index :type Integer))
  (bind (_returnvalue _dataasset) (`/Game/Core/GGJ_FunctionLibrary.Get Turret Data Asset` Index))
  (if _returnvalue
    (bind _output_get (set `self.Data Asset` _dataasset))
    (`StaticMeshComponent.SetStaticMesh` (`self.Mesh`) (`/Game/DataAsset/Turret/PDA_Turret.Mesh` _output_get))
    (`SceneComponent.SetRelativeScale3D` (`self.Decal Area`) (`/Game/DataAsset/Turret/PDA_Turret.Get Mesh Area` _output_get))
    (`MaterialInstanceDynamic.SetScalarParameterValue` (`self.Material Area`) "Size Lines" (`/Game/DataAsset/Turret/PDA_Turret.Get Shader SizeLines` _output_get))))

(event `self.ReceivePointDamage`
  (params (Damage :type "Float (single-precision)") (DamageType :type "DamageType Object Reference") (HitLocation :type "Vector Structure") (HitNormal :type "Vector Structure") (HitComponent :type "PrimitiveComponent Object Reference") (BoneName :type Name) (ShotFromDirection :type "Vector Structure") (InstigatedBy :type "Controller Object Reference") (DamageCauser :type "Actor Object Reference") (HitInfo :type "HitResult Structure (by ref)"))
  (bind _output_get (set `self.CurrentHealth` (- (`self.CurrentHealth`) Damage)))
  (if (<= _output_get 0.0)
    (`self.TowerDeath`)))

(event `TowerDeath`
  (`NiagaraFunctionLibrary.SpawnSystemAtLocation` "/Game/VFX/MysticWisps/NS_TurretDestroy.NS_TurretDestroy" (`self.K2_GetActorLocation`))
  (`self.K2_DestroyActor`))

(event `/Game/Core/BPI_Selection.BranchWidth`
  (bind _branch (`self.Branch`))
  (`/Engine/EditorBlueprintResources/StandardMacros.IsValid` _branch
    (:`Is Valid`
      (`/Game/BranchNiagara/BP_Branch.IncrementRootWidth` _branch))))

(event `/Game/Core/BPI_Selection.SetBranch`
  (params (Branch :type "/Game/BranchNiagara/BP_Branch Object Reference"))
  (set `self.Branch` Branch))

(event `/Game/Core/BPI_Selection.ActivateTurret`
  (`KismetSystemLibrary.Delay` 1.75)
  (`self.SetActorHiddenInGame` false))

(event `/Game/Core/BPI_Selection.Highlight`
  (bind _material_mesh (`self.Material Mesh`))
  (`MaterialInstanceDynamic.SetScalarParameterValue` _material_mesh "Highlight" 1.0)
  (`KismetSystemLibrary.RetriggerableDelay` 0.02)
  (`MaterialInstanceDynamic.SetScalarParameterValue` _material_mesh "Highlight" 0.0))

(fn `Get PDA`
  (returns (ReturnValue :type "/Game/DataAsset/Turret/PDA_Turret Object Reference"))
  (return (`self.Data Asset`)))

(fn `GetWeight`
  (returns (W :type Integer))
  (return (`self.Weight`)))

(fn `SetWeight`
  (params (W :type Integer))
  (set `self.Weight` W)
  (return))

(fn `Try Selection`
  (returns (ReturnValue :type Boolean))
  (`self.Change Selection State` true)
  (return true))

(fn `UserConstructionScript`)