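; Area-of-effect tower that damages every BP_Enemy inside its sphere and destroys itself when point damage depletes its health.
; An overlap while HasEnemy is false sets the flag and starts Attack, which applies point damage to all enemies in range and re-calls itself every second.
; End overlap clears HasEnemy once no enemies remain, but Attack's branch is always true, so the loop never checks the flag or stops.
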(event `self.ReceiveBeginPlay`
  (set `self.CurrentHealth` (`self.MaxHealth`)))

(event `self.ReceivePointDamage`
  (params (Damage :type "Float (single-precision)") (DamageType :type "DamageType Object Reference") (HitLocation :type "Vector Structure") (HitNormal :type "Vector Structure") (HitComponent :type "PrimitiveComponent Object Reference") (BoneName :type Name) (ShotFromDirection :type "Vector Structure") (InstigatedBy :type "Controller Object Reference") (DamageCauser :type "Actor Object Reference") (HitInfo :type "HitResult Structure (by ref)"))
  (bind _output_get (set `self.CurrentHealth` (- (`self.CurrentHealth`) Damage)))
  (if (<= _output_get 0.0)
    (`self.K2_DestroyActor`)))

(event `self.Sphere_0.OnComponentBeginOverlap`
  (params (OverlappedComponent :type "PrimitiveComponent Object Reference") (OtherActor :type "Actor Object Reference") (OtherComp :type "PrimitiveComponent Object Reference") (OtherBodyIndex :type Integer) (bFromSweep :type Boolean) (SweepResult :type "HitResult Structure (by ref)"))
  (if (not (`self.bHasEnemy`))
    (set `self.bHasEnemy` true)
    (`self.attack`)))

(event `attack`
  (if true
    (for _array_element (`PrimitiveComponent.GetOverlappingActors` (`self.Sphere_0`) "/Game/Enemies/Enemies/BP_Enemy.BP_Enemy_C")
      (`GameplayStatics.ApplyPointDamage` _array_element (`self.damage`) (`KismetMathLibrary.MakeVector` 0.0) (`GameplayStatics.MakeHitResult` false) null self))
    (`KismetSystemLibrary.Delay` 1.0)
    (`self.attack`)))

(event `self.Sphere_0.OnComponentEndOverlap`
  (params (OverlappedComponent :type "PrimitiveComponent Object Reference") (OtherActor :type "Actor Object Reference") (OtherComp :type "PrimitiveComponent Object Reference") (OtherBodyIndex :type Integer))
  (if (not (`KismetArrayLibrary.Array_IsValidIndex` (`PrimitiveComponent.GetOverlappingActors` (`self.Sphere_0`) "/Game/Enemies/Enemies/BP_Enemy.BP_Enemy_C")))
    (set `self.bHasEnemy` false)))

(fn `UserConstructionScript`
  (`parent.UserConstructionScript`))