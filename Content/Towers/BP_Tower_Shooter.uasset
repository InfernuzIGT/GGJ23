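; Shooter tower actor that attacks one target at a time within its sphere and destroys itself when point damage depletes its health.
; The first non-tower overlap starts a self-repeating Attack loop: spawn a Niagara shot, apply delayed point damage, wait VelAttack, repeat without checking HasEnemy.
; Tick steers the effect's endpoint to the target while HasEnemy is set.
; When the target leaves, another overlapping BP_Enemy replaces it or HasEnemy clears.
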(event `self.ReceivePointDamage`
  (params (Damage :type "Float (single-precision)") (DamageType :type "DamageType Object Reference") (HitLocation :type "Vector Structure") (HitNormal :type "Vector Structure") (HitComponent :type "PrimitiveComponent Object Reference") (BoneName :type Name) (ShotFromDirection :type "Vector Structure") (InstigatedBy :type "Controller Object Reference") (DamageCauser :type "Actor Object Reference") (HitInfo :type "HitResult Structure (by ref)"))
  (bind _output_get (set `self.CurrentHealth` (- (`self.CurrentHealth`) Damage)))
  (if (<= _output_get 0.0)
    (`self.K2_DestroyActor`)))

(event `self.ReceiveBeginPlay`
  (set `self.CurrentHealth` (`self.MaxHealth`)))

(event `Attack`
  (bind _returnvalue (`NiagaraFunctionLibrary.SpawnSystemAtLocation` "/Game/Towers/NS_TowerShoot.NS_TowerShoot" (`self.K2_GetActorLocation`) (struct) (1.0 1.0 1.0) true false))
  (set `self.FX` _returnvalue)
  (`FXSystemComponent.SetVectorParameter` _returnvalue "EndLoc" (`self.K2_GetActorLocation` (`self.target`)))
  (`ActorComponent.Activate` _returnvalue false)
  (`KismetSystemLibrary.Delay` 0.75)
  (`GameplayStatics.ApplyPointDamage` (`self.target`) (`self.Damage`) (`KismetMathLibrary.MakeVector` 0.0) (`GameplayStatics.MakeHitResult` false) null self)
  (`KismetSystemLibrary.Delay` (`self.Vel_Attack`))
  (`self.Attack`))

(event `self.Sphere_0.OnComponentBeginOverlap`
  (params (OverlappedComponent :type "PrimitiveComponent Object Reference") (OtherActor :type "Actor Object Reference") (OtherComp :type "PrimitiveComponent Object Reference") (OtherBodyIndex :type Integer) (bFromSweep :type Boolean) (SweepResult :type "HitResult Structure (by ref)"))
  (if (`self.ActorHasTag` OtherActor "Tower")
    _
    (elif (not (`self.bHasEnemy`))
      (set `self.bHasEnemy` true)
      (set `self.target` OtherActor)
      (`self.Attack`))))

(event `ChangeTarget`
  (params (NewTarget :type "Actor Object Reference"))
  (set `self.target` NewTarget))

(event `self.ReceiveTick`
  (params (DeltaSeconds :type "Float (single-precision)"))
  (`parent.ReceiveTick` DeltaSeconds)
  (if (`self.bHasEnemy`)
    (`FXSystemComponent.SetVectorParameter` (`self.FX`) "EndLoc" (`self.K2_GetActorLocation` (`self.target`)))))

(event `self.Sphere_0.OnComponentEndOverlap`
  (params (OverlappedComponent :type "PrimitiveComponent Object Reference") (OtherActor :type "Actor Object Reference") (OtherComp :type "PrimitiveComponent Object Reference") (OtherBodyIndex :type Integer))
  (bind _overlappingactors (`PrimitiveComponent.GetOverlappingActors` (`self.Sphere_0`) "/Game/Enemies/Enemies/BP_Enemy.BP_Enemy_C"))
  (if (== OtherActor (`self.target`))
    (if (`KismetArrayLibrary.Array_IsValidIndex` _overlappingactors)
      (`self.ChangeTarget` (`|GetArrayItem` _overlappingactors))
      (else
        (set `self.bHasEnemy` false)))))

(fn `UserConstructionScript`
  (`parent.UserConstructionScript`))