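; BP_Tower_view is a tower actor with health that can be destroyed by damage.
; It fills current health from its maximum on BeginPlay, then subtracts each point damage hit and destroys itself at zero or below.
; Before destruction it looks up BP_MasterController but makes no use of the result.
; The Sphere overlap event is empty, and the construction script only calls its parent.
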(event `self.ReceiveBeginPlay`
  ;[1 1 1] health
  (set `self.CurrentHealth` (`self.MaxHealth`)))

(event `self.ReceivePointDamage`
  (params (Damage :type "Float (single-precision)") (DamageType :type "DamageType Object Reference") (HitLocation :type "Vector Structure") (HitNormal :type "Vector Structure") (HitComponent :type "PrimitiveComponent Object Reference") (BoneName :type Name) (ShotFromDirection :type "Vector Structure") (InstigatedBy :type "Controller Object Reference") (DamageCauser :type "Actor Object Reference") (HitInfo :type "HitResult Structure (by ref)"))
  ;[1 1 1] destroy
  (bind _output_get (set `self.CurrentHealth` (- (`self.CurrentHealth`) Damage)))
  (if (<= _output_get 0.0)
    (`GameplayStatics.GetActorOfClass` "/Game/MasterController/BP_MasterController.BP_MasterController_C")
    (`self.K2_DestroyActor`)))

(event `self.Sphere.OnComponentBeginOverlap`
  (params (OverlappedComponent :type "PrimitiveComponent Object Reference") (OtherActor :type "Actor Object Reference") (OtherComp :type "PrimitiveComponent Object Reference") (OtherBodyIndex :type Integer) (bFromSweep :type Boolean) (SweepResult :type "HitResult Structure (by ref)")))

(fn `UserConstructionScript`
  (`parent.UserConstructionScript`))