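; BP_Boss is a boss enemy that attacks towers, extending a parent enemy's Attack event.
; Its sphere overlap triggers Attack for actors tagged Tower but not Sapling.
; Attack stops movement, applies point damage to CurrentTarget, spawns a Niagara effect ahead of the boss, then calls itself again after a cooldown.
; Tick adds no behavior, and a distance-based attack check is left disconnected.
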(event `self.ReceiveTick`
  (params (DeltaSeconds :type "Float (single-precision)"))
  (`parent.ReceiveTick` DeltaSeconds)
  (if (`self.bTargetBase`)
    _))

(event `self.Attack`
  (`parent.Attack`)
  (if (not (`self.bAttackOnCooldown`))
    (set `self.bAttackOnCooldown` true)
    (`CharacterMovementComponent.SetMovementMode` (`self.CharacterMovement`) "MOVE_None" 0)
    (`GameplayStatics.ApplyPointDamage` (`self.CurrentTarget`) (`self.Damage`) (`KismetMathLibrary.MakeVector` 0.0) (`GameplayStatics.MakeHitResult` false) null self)
    (`NiagaraFunctionLibrary.SpawnSystemAtLocation` "/Game/Enemies/Enemies/NS_BossAttack.NS_BossAttack" (+ (`self.K2_GetActorLocation`) (* (`KismetMathLibrary.GetForwardVector` (`self.K2_GetActorRotation`)) 600.0)))
    (`KismetSystemLibrary.Delay` (`self.AttackCooldown`))
    (set `self.bAttackOnCooldown` false)
    (`self.Attack`)))

(event `self.Sphere.OnComponentBeginOverlap`
  (params (OverlappedComponent :type "PrimitiveComponent Object Reference") (OtherActor :type "Actor Object Reference") (OtherComp :type "PrimitiveComponent Object Reference") (OtherBodyIndex :type Integer) (bFromSweep :type Boolean) (SweepResult :type "HitResult Structure (by ref)"))
  (if (and (`self.ActorHasTag` OtherActor "Tower") (not (`self.ActorHasTag` OtherActor "Sapling")))
    (`self.Attack`)))

(fn `UserConstructionScript`
  (`parent.UserConstructionScript`))