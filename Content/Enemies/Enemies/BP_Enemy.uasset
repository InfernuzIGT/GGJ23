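; Enemy character with an evil aura effect that walks toward a target point and tracks its own health.
; Each tick it steers and yaws toward a stored location until Attack halts it.
; TargetCollision overlaps divert it from the base to non-Sapling actors; when its target leaves, it takes another overlapping target or heads back to world origin.
; Point damage reduces health, and death notifies the master controller before destroying the actor.
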(event `self.ReceiveBeginPlay`
  (bind _capsulecomponent (`self.CapsuleComponent`))
  (set `self.CurrentHealth` (`self.MaxHealth`))
  (set `CharacterMovementComponent.MaxWalkSpeed` (`self.MovementSpeed`) (`self.CharacterMovement`))
  (`NiagaraFunctionLibrary.SpawnSystemAttached` "/Game/Enemies/Enemies/NS_EnemiesEvilAura.NS_EnemiesEvilAura" _capsulecomponent "None" (`SceneComponent.K2_GetComponentLocation` _capsulecomponent) (struct) "KeepWorldPosition"))

(event `self.ReceiveTick`
  (params (DeltaSeconds :type "Float (single-precision)"))
  (`self.MoveToPoint`))

(event `MoveToPoint`
  (bind _returnvalue (`self.K2_GetActorLocation`))
  (bind _todirection (`self.ToDirection`))
  (bind (_returnvalue_roll _returnvalue_pitch _returnvalue_yaw) (`KismetMathLibrary.BreakRotator` (`KismetMathLibrary.FindLookAtRotation` _returnvalue _todirection)))
  (if (not (`self.bMovementStop`))
    (`self.AddMovementInput` (`KismetMathLibrary.GetDirectionUnitVector` _returnvalue _todirection))
    (`self.K2_SetActorRotation` (`KismetMathLibrary.MakeRotator` 0.0 0.0 _returnvalue_yaw))))

(event `self.ReceivePointDamage`
  (params (Damage :type "Float (single-precision)") (DamageType :type "DamageType Object Reference") (HitLocation :type "Vector Structure") (HitNormal :type "Vector Structure") (HitComponent :type "PrimitiveComponent Object Reference") (BoneName :type Name) (ShotFromDirection :type "Vector Structure") (InstigatedBy :type "Controller Object Reference") (DamageCauser :type "Actor Object Reference") (HitInfo :type "HitResult Structure (by ref)"))
  (bind _output_get (set `self.CurrentHealth` (- (`self.CurrentHealth`) Damage)))
  (if (<= _output_get 0.0)
    (`self.Death`)))

(event `Death`
  (`/Game/MasterController/BP_MasterController.EnemyDeath` (`self.MasterControllerRef`))
  (`self.K2_DestroyActor`))

(event `ChangeTarget`
  (params (NewTarget :type "Actor Object Reference"))
  (bind _output_get (set `self.CurrentTarget` NewTarget))
  (set `self.ToDirection` (`self.K2_GetActorLocation` _output_get)))

(event `self.TargetCollision.OnComponentBeginOverlap`
  (params (OverlappedComponent :type "PrimitiveComponent Object Reference") (OtherActor :type "Actor Object Reference") (OtherComp :type "PrimitiveComponent Object Reference") (OtherBodyIndex :type Integer) (bFromSweep :type Boolean) (SweepResult :type "HitResult Structure (by ref)"))
  (if (`self.ActorHasTag` OtherActor "Sapling")
    _
    (elif (`self.bTargetBase`)
      (set `self.bTargetBase` false)
      (`self.ChangeTarget` OtherActor))))

(event `self.TargetCollision.OnComponentEndOverlap`
  (params (OverlappedComponent :type "PrimitiveComponent Object Reference") (OtherActor :type "Actor Object Reference") (OtherComp :type "PrimitiveComponent Object Reference") (OtherBodyIndex :type Integer))
  (bind _overlappingactors (`PrimitiveComponent.GetOverlappingActors` (`self.TargetCollision`) "/Game/Enemies/Enemies/BP_EnemyTargetTest.BP_EnemyTargetTest_C"))
  (bind _output (`|GetArrayItem` _overlappingactors))
  (if (== (`self.CurrentTarget`) OtherActor)
    (if (`KismetArrayLibrary.Array_IsValidIndex` _overlappingactors)
      (if (`self.ActorHasTag` _output "Sapling")
        (set `self.bTargetBase` true :!label _label)
        (set `self.ToDirection` (0.0 0.0 0.0))
        (set `self.bMovementStop` false)
        (else
          (`self.ChangeTarget` _output)
          (set `self.bMovementStop` false)))
      (else
        (goto _label)))))

(event `Attack`
  (set `self.bMovementStop` true))

(fn `UserConstructionScript`)