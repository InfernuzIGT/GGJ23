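; Ranged enemy Blueprint that damages its current target from a distance, extending a parent class's Tick and Attack events.
; Each Tick, while TargetBase is not set, it measures the distance to CurrentTarget and calls Attack when within AttackRange.
; Attack applies point damage directly, with no projectile or trace, then uses a boolean and Delay as a cooldown gate.
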(event `self.ReceiveTick`
  (params (DeltaSeconds :type "Float (single-precision)"))
  (`parent.ReceiveTick` DeltaSeconds)
  (if (`self.bTargetBase`)
    _
    (elif (<= (`KismetMathLibrary.Vector_Distance` (`self.K2_GetActorLocation`) (`self.K2_GetActorLocation` (`self.CurrentTarget`))) (`self.AttackRange`))
      (`self.Attack`))))

(event `self.Attack`
  (`parent.Attack`)
  (if (not (`self.bAttackOnCooldown`))
    (set `self.bAttackOnCooldown` true)
    (`GameplayStatics.ApplyPointDamage` (`self.CurrentTarget`) (`self.Damage`) (`KismetMathLibrary.MakeVector` 0.0) (`GameplayStatics.MakeHitResult` false) null self)
    (`KismetSystemLibrary.Delay` (`self.AttackCooldown`))
    (set `self.bAttackOnCooldown` false)))

(fn `UserConstructionScript`
  (`parent.UserConstructionScript`))