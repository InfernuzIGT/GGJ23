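; Actor that registers itself with BP_RenderCamera as an actor to render and marks its location on the RT_Fog render target, apparently for a fog mask.
; One second after BeginPlay, it draws a small polygon on that target at its projected screen position and sizes its capsule from MaxSize.X.
; A timeline then scales the SMRender mesh from unit scale up to MaxSize.
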(event `self.ReceiveBeginPlay`
  (bind _returnvalue (* (/ (.x (`self.MaxSize`)) 2.0) 100.0))
  (`KismetSystemLibrary.Delay` 1.0)
  (bind _returnvalue_2 (`GameplayStatics.GetActorOfClass` "/Game/Core/RenderCamera/BP_RenderCamera.BP_RenderCamera_C"))
  (`/Game/Core/RenderCamera/BP_RenderCamera.Add Actor to Render` _returnvalue_2 self)
  (bind (_canvas _size) (`KismetRenderingLibrary.BeginDrawCanvasToRenderTarget` "/Game/Core/RenderCamera/RT_Fog.RT_Fog"))
  (`Canvas.K2_DrawPolygon` _canvas null (* _size (`GameplayStatics.ProjectWorldToScreen` null (`self.K2_GetActorLocation`) true)) (10.0 10.0) 16 (struct :`R` 1.0 :`G` 1.0 :`B` 1.0 :`A` 1.0))
  (`CapsuleComponent.SetCapsuleSize` (`self.Capsule`) _returnvalue _returnvalue true)
  (bind (_direction _newtrack_0) (`Timeline|Timeline_0` :!via `PlayFromStart`)
    (:`Update`
      (`SceneComponent.SetWorldScale3D` (`self.SM_Render`) (`KismetMathLibrary.VLerp` (1.0 1.0 1.0) (`self.MaxSize`) _newtrack_0)))))

(fn `UserConstructionScript`)