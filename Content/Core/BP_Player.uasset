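; Player pawn for a root-growing tower defense, handling movement, mana, HUD messages, sapling progress and game over.
; Clicking a selectable root enters placement mode, where a cursor previews the turret picked by number key or HUD, using its data asset.
; Tick tints the area decal by range from the selected root and sphere-traces for crowding.
; A valid, affordable click spends mana and spawns the turret with the parent's weight plus one.
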(event `self.ReceiveBeginPlay`
  (bind _returnvalue (`GameplayStatics.GetPlayerController` 0))
  (`|ExecutionSequence`
    (:`then_0`
      (set `PlayerController.bShowMouseCursor` true _returnvalue)
      (`WidgetBlueprintLibrary.SetInputMode_GameAndUIEx` _returnvalue null "DoNotLock" false))
    (:`then_1`
      (bind _returnvalue_2 (`|CreateWidget` "/Game/Widgets/HUD/WBP_HUD.WBP_HUD_C"))
      (bind _output_get (set `self.Widget HUD` _returnvalue_2))
      (`UserWidget.AddToViewport` _output_get 0)
      (add `/Game/Widgets/HUD/WBP_HUD.OnSelectTurret` _output_get (delegate `OnSelectTurret_Event`)))
    (:`then_2`
      (set `self.StartLocation` (`self.K2_GetActorLocation`))
      (bind _returnvalue_3 (`DecalComponent.CreateDynamicMaterialInstance` (`self.Decal Area`)))
      (set `self.Material Area` _returnvalue_3)
      (`self.Select Turret` (`self.LastSelectionIndex`))
      (`self.Change Cursor Visibility` false))
    (:`then_3`
      (`self.AddCurrency` 250))))

(event `OnSelectTurret_Event`
  (params (Index :type Integer))
  (`self.Select Turret` Index))

(event `Change Cursor Visibility`
  (params (bVisible :type Boolean))
  (`SceneComponent.SetVisibility` (`self.Cursor`) bVisible true))

(event `Select Turret`
  (params (Index :type Integer))
  (bind _output_get (set `self.LastSelectionIndex` Index))
  (bind (_returnvalue _dataasset) (`/Game/Core/GGJ_FunctionLibrary.Get Turret Data Asset` _output_get))
  (if _returnvalue
    (`StaticMeshComponent.SetStaticMesh` (`self.ST_Turret`) (`/Game/DataAsset/Turret/PDA_Turret.Mesh` _dataasset))
    (`SceneComponent.SetRelativeScale3D` (`self.Decal Area`) (`/Game/DataAsset/Turret/PDA_Turret.Get Mesh Area` _dataasset))
    (`MaterialInstanceDynamic.SetScalarParameterValue` (`self.Material Area`) "Size Area" (`/Game/DataAsset/Turret/PDA_Turret.Get Shader SizeArea` _dataasset))
    (set `self.TempClassToSpawn` (`/Game/DataAsset/Turret/PDA_Turret.Class` _dataasset))
    (set `self.TempTurretCost` (`/Game/DataAsset/Turret/PDA_Turret.Cost` _dataasset))))

(event `self.ReceiveTick`
  (params (DeltaSeconds :type "Float (single-precision)"))
  (bind (_bblockinghit _binitialoverlap _time _distance _location) (`GameplayStatics.BreakHitResult` (`PlayerController.GetHitResultUnderCursorByChannel` (`GameplayStatics.GetPlayerController` 0) "TraceTypeQuery1" false)))
  (bind _returnvalue (> (`KismetMathLibrary.Vector_Distance` _location (`self.K2_GetActorLocation` (`self.CurrentSelection`))) (`/Game/DataAsset/Turret/PDA_Turret.Area` (`self.CurrentSelectionPDA`))))
  (`SceneComponent.K2_SetWorldLocation` (`self.Cursor`) _location false false)
  (if (`|EnumEquality` (`self.CurrentSelectionState`) "NewEnumerator1")
    (`MaterialInstanceDynamic.SetVectorParameterValue` (`self.Material Area`) "Color" (select `bool` _returnvalue :`false` (struct :`G` 1.0 :`A` 1.0) :`true` (struct :`R` 1.0 :`A` 1.0) :!type "LinearColor Structure"))
    (set `self.bLocationInvalid` _returnvalue)
    (bind (_outhit _returnvalue_2) (`KismetSystemLibrary.SphereTraceSingleForObjects` :`Start` _location :`End` _location :`Radius` 500.0 :`ObjectTypes` (`|MakeArray` "ObjectTypeQuery7" :!type "EObjectTypeQuery Enum") :`DrawDebugType` "ForOneFrame"))
    (set `self.bLocationInvalidCloseTree` _returnvalue_2)))

(event `AddCurrency`
  (params (Add :type Integer))
  (bind _output_get (set `self.Currency` (+ (`self.Currency`) Add)))
  (`/Game/Widgets/HUD/WBP_HUD.UpdateCurrency` (`self.Widget HUD`) _output_get))

(event `GameOver`
  (`/Game/Widgets/HUD/WBP_HUD.GameOver` (`self.Widget HUD`)))

(event `AddSaplingFound`
  (bind _output_get (set `self.SaplingFound` (+ (`self.SaplingFound`) 1)))
  (if (== _output_get 3)
    (`/Game/Widgets/HUD/WBP_HUD.ShowWarningMessage` (`self.Widget HUD`) "All sapling found!" 6.0)
    (`KismetSystemLibrary.Delay` 3.0)
    (`/Game/Widgets/HUD/WBP_HUD.ShowWarningMessage` (`self.Widget HUD`) "Something evil is coming!" 6.0)))

(event `Key|One`
  (params (Key :type "Key Structure"))
  (:`Pressed`
    (`self.Select Turret` 1)))

(event `InputAxis|MoveForward` :overrideparent false
  (params (AxisValue :type "Float (single-precision)"))
  (`self.AddMovementInput` (`self.GetActorForwardVector`) AxisValue))

(event `Key|Two`
  (params (Key :type "Key Structure"))
  (:`Pressed`
    (`self.Select Turret` 2)))

(event `Key|Three`
  (params (Key :type "Key Structure"))
  (:`Pressed`
    (`self.Select Turret` 3)))

(event `InputAxis|MoveRight` :overrideparent false
  (params (AxisValue :type "Float (single-precision)"))
  (`self.AddMovementInput` (`self.GetActorRightVector`) AxisValue))

(event `Key|Four`
  (params (Key :type "Key Structure"))
  (:`Pressed`
    (`self.Select Turret` 4)))

(event `Key|SpaceBar`
  (params (Key :type "Key Structure"))
  (:`Pressed`
    (`self.K2_SetActorLocation` (`self.StartLocation`))))

(event `Key|Escape`
  (params (Key :type "Key Structure"))
  (:`Pressed`
    (switch `/Game/Core/E_SelectionState` (`self.CurrentSelectionState`) :!label _label
      (:`NewEnumerator1`
        (`self.Clear Selection`)))))

(event `Key|RightMouseButton`
  (params (Key :type "Key Structure"))
  (:`Pressed`
    (goto _label)))

(event `Key|LeftMouseButton`
  (params (Key :type "Key Structure"))
  (bind (_hitresult _returnvalue) (`PlayerController.GetHitResultUnderCursorByChannel` (`GameplayStatics.GetPlayerController` 0) "TraceTypeQuery1" false))
  (bind (_bblockinghit _binitialoverlap _time _distance _location _impactpoint _normal _impactnormal _physmat _hitactor) (`GameplayStatics.BreakHitResult` _hitresult))
  (:`Pressed`
    (switch `/Game/Core/E_SelectionState` (`self.CurrentSelectionState`)
      (:`NewEnumerator0`
        (if _returnvalue
          (bind _returnvalue_2 (message `/Game/Core/BPI_Selection.Try Selection` _hitactor))
          (if _returnvalue_2
            (set `self.CurrentSelectionState` "NewEnumerator1")
            (bind _output_get (set `self.CurrentSelection` _hitactor))
            (bind _returnvalue_3 (message `/Game/Core/BPI_Selection.Get PDA` _output_get))
            (set `self.CurrentSelectionPDA` _returnvalue_3)
            (`/Game/Widgets/HUD/WBP_HUD.Change Selection State` (`self.Widget HUD`) true)
            (`self.Select Turret` (`self.LastSelectionIndex`))
            (`self.Change Cursor Visibility` true))))
      (:`NewEnumerator1`
        (if (`self.bLocationInvalid`)
          (`/Game/Widgets/HUD/WBP_HUD.ShowWarningMessage` (`self.Widget HUD`) "Location far away from a root!" 5.0)
          (elif (`self.bLocationInvalidCloseTree`)
            (`/Game/Widgets/HUD/WBP_HUD.ShowWarningMessage` (`self.Widget HUD`) "Location too close from another root!" 5.0)
            (elif (<= (`self.TempTurretCost`) (`KismetMathLibrary.Conv_IntToDouble` (`self.Currency`)))
              (`self.AddCurrency` (`KismetMathLibrary.FTrunc` (* -1 (`self.TempTurretCost`))))
              (bind _returnvalue_4 (`|SpawnActorFromClass` (`self.TempClassToSpawn`) (`KismetMathLibrary.MakeTransform` _location) "Undefined" "OverrideRootScale" null null))
              (message `/Game/Core/BPI_Selection.Update Data` _returnvalue_4 (`self.LastSelectionIndex`))
              (bind _w (message `/Game/Core/BPI_Selection.GetWeight` (`self.CurrentSelection`)))
              (message `/Game/Core/BPI_Selection.SetWeight` _returnvalue_4 (+ _w 1))
              (`self.Clear Selection`)
              (else
                (`/Game/Widgets/HUD/WBP_HUD.ShowWarningMessage` (`self.Widget HUD`) "Not enough mana for a root!" 5.0)))))))))

(event `Clear Selection`
  (set `self.CurrentSelectionState` "NewEnumerator0")
  (message `/Game/Core/BPI_Selection.Remove Selection` (`self.CurrentSelection`))
  (set `self.CurrentSelection` null)
  (set `self.CurrentSelectionPDA` null)
  (`/Game/Widgets/HUD/WBP_HUD.Change Selection State` (`self.Widget HUD`) false)
  (`self.Change Cursor Visibility` false))

(fn `UserConstructionScript`)