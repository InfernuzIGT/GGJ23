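; BP_Debug is a debug actor that can be selected and can display a turret mesh chosen by index.
; On BeginPlay it creates a dynamic material on its Sphere component and starts unselected.
; TrySelection and RemoveSelection route through ChangeSelectionState, which sets the Color parameter to green or white.
; UpdateData looks up a turret data asset and, if found, swaps the Sphere's static mesh to that asset's mesh.
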(event `Change Selection State`
  (params (bIsSelected :type Boolean))
  (`MaterialInstanceDynamic.SetVectorParameterValue` (`self.Material`) "Color" (select `bool` bIsSelected :`false` (struct :`R` 1.0 :`G` 1.0 :`B` 1.0 :`A` 1.0) :`true` (struct :`G` 1.0 :`A` 1.0) :!type "LinearColor Structure")))

(event `self.ReceiveBeginPlay`
  (bind _sphere (`self.Sphere`))
  (bind _returnvalue (`PrimitiveComponent.CreateDynamicMaterialInstance` _sphere 0 (`PrimitiveComponent.GetMaterial` _sphere 0) "None"))
  (set `self.Material` _returnvalue)
  (`self.Change Selection State` false))

(event `/Game/Core/BPI_Selection.Remove Selection`
  (`self.Change Selection State` false))

(event `/Game/Core/BPI_Selection.Update Data`
  (params (Index :type Integer))
  (bind (_returnvalue _dataasset) (`/Game/Core/GGJ_FunctionLibrary.Get Turret Data Asset` Index))
  (if _returnvalue
    (`StaticMeshComponent.SetStaticMesh` (`self.Sphere`) (`/Game/DataAsset/Turret/PDA_Turret.Mesh` _dataasset))))

(fn `Try Selection`
  (returns (ReturnValue :type Boolean))
  (`self.Change Selection State` true)
  (return true))

(fn `UserConstructionScript`)